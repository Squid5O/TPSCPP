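; Enemy state machine that runs on Tick for its owning BP_Enemy, with Idle, Move and Attack states.
; Idle caches the player character as target and the owner as self, then switches to Move.
; Move steers toward the target until within AttackDist, then switches to Attack.
; Attack is a placeholder print after a two-second Delay, returning to Idle when the target's 2D distance exceeds AttackDist.
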(event `self.ReceiveTick`
  (params (DeltaSeconds :type "Float (single-precision)"))
  (bind _returnvalue (`GameplayStatics.GetPlayerCharacter` 0))
  (bind _me (`self.Me`))
  (bind _returnvalue_2 (- (`Actor.K2_GetActorLocation` (`self.target`)) (`Actor.K2_GetActorLocation` _me)))
  (switch `/Game/Blueprints/temp/BP_EEnmeyState` (`self.state`)
    (:`NewEnumerator0`
      ;[1 1 1] Idle: 주인공을 찾아서 목적지를 기억하고 싶다. 목적지가 있다면 이동 상태로 전의
      (`/Engine/EditorBlueprintResources/StandardMacros.IsValid` _returnvalue
        (:`Is Valid`
          (set `self.target` _returnvalue)
          (bind _asbp_enemy (cast `/Game/Blueprints/BP_Enemy` (`self.GetOwner`)))
          (set `self.Me` _asbp_enemy)
          (set `self.state` "NewEnumerator1"))))
    (:`NewEnumerator1`
      ;[1 1 1] Move : 목적지를 향해서 이동하고 싶다. 만약 목적지와의 거리가 3m 이내라면 공격상태로 전이하고 싶다.
      (`Pawn.AddMovementInput` _me _returnvalue_2 1.0 false)
      (if (< (`KismetMathLibrary.VSize` _returnvalue_2) (`self.attackDist`))
        (set `self.state` "NewEnumerator2")))
    (:`NewEnumerator2`
      ;[1 1 1] Attack : 공격을 하고 2초 대기했다가 다시 공격하고 싶다. 만약 공격을 하려고 할때 목적지와의 거리를 3m를 초과한다면 이동상태로 전이하고 싶어
      (`KismetSystemLibrary.Delay` 2.0)
      (`KismetSystemLibrary.PrintString` "Hello" true true (struct :`G` 0.66 :`B` 1.0 :`A` 1.0) 10.0)
      (if (> (`KismetMathLibrary.Vector_Distance2D` (`Actor.K2_GetActorLocation` (`self.target`)) (`Actor.K2_GetActorLocation` (`self.Me`))) (`self.attackDist`))
        (set `self.state` "NewEnumerator0")))))